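; Player controller that shows on-screen instructions and user info and handles account login and logout from input.
; BeginPlay creates the W_Instructions and W_UserInfo widgets and adds both to the viewport.
; The Login and Logout actions, on release, send a login request with hardcoded localhost AccountPortal credentials or a logout request, then print the returned result on screen.
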(event `self.ReceiveBeginPlay`
  (`|ExecutionSequence`
    (:`then_0`
      (bind _returnvalue (`|CreateWidget` "/Game/Widgets/W_Instructions.W_Instructions_C" self))
      (bind _output_get (set `self.Instructions` _returnvalue))
      (`UserWidget.AddToViewport` _output_get 0))
    (:`then_1`
      (bind _returnvalue_2 (`|CreateWidget` "/Game/Widgets/W_UserInfo.W_UserInfo_C" self))
      (bind _output_get_2 (set `self.UserInfo` _returnvalue_2))
      (`UserWidget.AddToViewport` _output_get_2 0))))

(event `self.ReceiveTick`
  (params (DeltaSeconds :type "Float (single-precision)")))

(event `InputAction|Login`
  (params (Key :type "Key Structure"))
  (:`Released`
    (bind _returnvalue (`self.RequestLogin` "localhost:11205" "xm" "AccountPortal"))
    (`KismetSystemLibrary.PrintString` (`KismetStringLibrary.Concat_StrStr` "Login Request: " (`KismetStringLibrary.Conv_BoolToString` _returnvalue)) true true (struct :`R` 1.0 :`G` 0.797706 :`A` 1.0) 10.0)))

(event `InputAction|Logout`
  (params (Key :type "Key Structure"))
  (:`Released`
    (bind _returnvalue (`self.RequestLogout`))
    (`KismetSystemLibrary.PrintString` (`KismetStringLibrary.Concat_StrStr` "Logout Request: " (`KismetStringLibrary.Conv_BoolToString` _returnvalue)) true true (struct :`R` 1.0 :`G` 0.797706 :`A` 1.0) 10.0)))

(fn `UserConstructionScript`)